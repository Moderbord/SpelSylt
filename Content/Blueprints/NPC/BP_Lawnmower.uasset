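; BP_Lawnmower is an AI-controlled lawnmower NPC that respawns the Tomte player character when its body overlaps them.
; It binds to its AI controller's chase-mode event to switch the spotlight red while chasing and yellow otherwise.
; Each tick it aligns itself to the floor normal while keeping its yaw, and spins its four wheels in proportion to movement speed.
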(event `On Target Changed`
  (params (Target :type "Vector Structure")))

(event `self.ReceiveBeginPlay`
  (set `self.PlayerStart` (`SceneComponent.K2_GetComponentToWorld` (`Actor.RootComponent` (`GameplayStatics.GetPlayerPawn` 0))))
  (bind _asbp_aicontroller (cast `/Game/Blueprints/NPC/AI/BP_AIController` (`AIBlueprintHelperLibrary.GetAIController` self)))
  (`|ExecutionSequence`
    (:`then_0`
      (add `/Game/Blueprints/NPC/AI/BP_AIController.TargetChanged` _asbp_aicontroller (delegate `On Target Changed`)))
    (:`then_1`
      (add `/Game/Blueprints/NPC/AI/BP_AIController.ChaseModeChanged` _asbp_aicontroller (delegate `On Chase Mode Changed`)))))

(event `On Chase Mode Changed`
  (params (IsChasing :type Boolean))
  (`LightComponent.SetLightColor` (`self.SpotLight`) (`KismetMathLibrary.SelectColor` (struct :`R` 1.0 :`A` 1.0) (struct :`R` 1.0 :`G` 1.0 :`A` 1.0) IsChasing) true))

(event `self.ReceiveActorBeginOverlap`
  (params (OtherActor :type "Actor Object Reference")))

(event `self.ReceiveTick`
  (params (DeltaSeconds :type "Float (single-precision)"))
  (bind (_currentfloor_bblockinghit _currentfloor_bwalkablefloor _currentfloor_blinetrace _currentfloor_floordist _currentfloor_linedist _currentfloor_hitresult) (break `FindFloorResult` (`CharacterMovementComponent.CurrentFloor` (`self.CharacterMovement`))))
  (bind (_bblockinghit _binitialoverlap _time _distance _location _impactpoint _normal _impactnormal) (`GameplayStatics.BreakHitResult` _currentfloor_hitresult))
  (`|ExecutionSequence`
    (:`then_0`
      (if _bblockinghit
        (`self.K2_SetActorRotation` (`KismetMathLibrary.MakeRotFromZX` _impactnormal (`KismetMathLibrary.GetForwardVector` (`KismetMathLibrary.MakeRotator` (.roll (`self.K2_GetActorRotation`)) 0.0 (.yaw (`self.K2_GetActorRotation`))))))))
    (:`then_1`
      (`SceneComponent.K2_AddRelativeRotation` (`self.RLOffset`) (`KismetMathLibrary.MakeRotator` 0.0 (* (`KismetMathLibrary.VSize` (`CharacterMovementComponent.GetLastUpdateVelocity` (`self.CharacterMovement`))) (`self.WheelSpeed`))) false false)
      (`SceneComponent.K2_AddRelativeRotation` (`self.FROffset`) (`KismetMathLibrary.MakeRotator` 0.0 (* (`KismetMathLibrary.VSize` (`CharacterMovementComponent.GetLastUpdateVelocity` (`self.CharacterMovement`))) (`self.WheelSpeed`))) false false)
      (`SceneComponent.K2_AddRelativeRotation` (`self.FLOffset`) (`KismetMathLibrary.MakeRotator` 0.0 (* (`KismetMathLibrary.VSize` (`CharacterMovementComponent.GetLastUpdateVelocity` (`self.CharacterMovement`))) (`self.WheelSpeed`))) false false)
      (`SceneComponent.K2_AddRelativeRotation` (`self.RROffset`) (`KismetMathLibrary.MakeRotator` 0.0 (* (`KismetMathLibrary.VSize` (`CharacterMovementComponent.GetLastUpdateVelocity` (`self.CharacterMovement`))) (`self.WheelSpeed`))) false false))))

(event `self.Lawmower_body.OnComponentBeginOverlap`
  (params (OverlappedComponent :type "PrimitiveComponent Object Reference") (OtherActor :type "Actor Object Reference") (OtherComp :type "PrimitiveComponent Object Reference") (OtherBodyIndex :type Integer) (bFromSweep :type Boolean) (SweepResult :type "HitResult Structure (by ref)"))
  (bind _asbp_tomte_character (cast `/Game/Blueprints/Player/BP_TomteCharacter` OtherActor))
  (`/Game/Blueprints/Player/BP_TomteCharacter.Respawn` _asbp_tomte_character))

(fn `UserConstructionScript`)