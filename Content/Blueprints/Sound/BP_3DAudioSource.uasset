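; 3D audio source actor that simulates sound occlusion by static world geometry between itself and the player.
; On Tick, a Delay-throttled test runs a multi-object line trace from the source to just above the player pawn.
; Hit physical surfaces map to wood, metal, stone or default factors, which are multiplied together and inverted.
; The result drives an occlusion parameter on the AudioComponent, zeroed when unobstructed or disabled.
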(event `self.ReceiveBeginPlay`
  (set `self.Listener` (`GameplayStatics.GetPlayerPawn` 0)))

(event `self.ReceiveTick`
  (params (DeltaSeconds :type "Float (single-precision)"))
  (`self.OcclusionTest`))

(fn `SetLocations`
  (params (ListenerLocation :type "Vector Structure") (SourceLocation :type "Vector Structure"))
  (returns (Distance :type "Float (double-precision)"))
  (bind _output_get (set `self.ListenerLocation` ListenerLocation))
  (bind _output_get_2 (set `self.SourceLocation` SourceLocation))
  (return (`KismetMathLibrary.VSize` (- _output_get _output_get_2))))

(fn `SurfaceOcclusionModifier`
  (params (Selection :type "EPhysicalSurface Enum" :default "SurfaceType_Default"))
  (returns (Modifier :type "Float (double-precision)"))
  (locals (Factor :type "Float (double-precision)"))
  (switch `EPhysicalSurface` Selection
    (:`SurfaceType_Default`
      (set `local.Factor` 0.8))
    (:`SurfaceType1`
      (set `local.Factor` 0.4))
    (:`SurfaceType2`
      (set `local.Factor` 0.55))
    (:`SurfaceType3`
      (set `local.Factor` 0.7)))
  (return (`local.Factor`)))

(fn `TotalHitOcclusion`
  (params (Objects :type "Array of HitResult Structure"))
  (returns (Value :type "Float (double-precision)"))
  (locals (Occlusion :type "Float (double-precision)" :default 1.0))
  (for _array_element Objects
    (bind _modifier (`self.SurfaceOcclusionModifier` (`PhysicalMaterial.SurfaceType` (`.PhysMat` (`GameplayStatics.BreakHitResult` _array_element)))))
    (set `local.Occlusion` (* _modifier (`local.Occlusion`))))
  (return (- 1.0 (`local.Occlusion`))))

(fn `UserConstructionScript`)