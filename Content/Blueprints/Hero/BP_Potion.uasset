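; BP_Potion is a potion actor that the player drinks when it is taken, applying the effects of its ingredients.
; On BeginPlay it hands itself and its ingredient list to the label widget in its IngredientsWidget component.
; OnTake calls Consume, which constructs each ingredient class and applies it to the player's TomteCharacter, scaled by its share of the potion's volume.
; It then plays a Burp event attached to the player and destroys itself.
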(event `self.ReceiveBeginPlay`
  (bind _aslabel_widget (cast `/Game/Blueprints/Environment/Labels/Widgets/LabelWidget` (`WidgetComponent.GetWidget` (`self.IngredientsWidget`))))
  (set `/Game/Blueprints/Environment/Labels/Widgets/LabelWidget.Owner` self _aslabel_widget)
  (`/Game/Blueprints/Environment/Labels/Widgets/LabelWidget.UpdateList` _aslabel_widget (`self.Ingredients`)))

(event `/Game/Blueprints/Player/I_Grabbable.OnTake`
  (`self.Consume`))

(fn `Consume`
  (bind _returnvalue (`GameplayStatics.GetPlayerCharacter` 0))
  (for _array_element (`self.Ingredients`)
    (bind (_ingredient _volume) (break `/Game/Blueprints/Hero/Ingredients/IngredientPackage` _array_element))
    (bind _returnvalue_2 (`|GenericCreateObject` _ingredient self))
    (bind _astomte_character (cast `/Game/Blueprints/Player/TomteCharacter` _returnvalue))
    (`/Game/Blueprints/Hero/Ingredients/BP_IngredientBase.Consume` _returnvalue_2 _astomte_character (/ _volume (`self.Volume`))))
  (`FMODBlueprintStatics.PlayEventAttached` "/Game/FMOD/Events/Actors/Player/Burp/Burp.Burp" (`Actor.RootComponent` _returnvalue) "None" (0.0 0.0 0.0) "KeepRelativeOffset")
  (`self.K2_DestroyActor`))

(fn `UserConstructionScript`)