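; Cauldron actor that brews potions from dropped ingredients or potions, with wood adding heat and water extinguishing it.
; Contents merge into an indexed ingredient list that drives volume, blended color and a widget fading with player distance.
; Each tick interpolates visuals, cools toward ambient, and tests one random recipe and ingredient for temperature-based crafting or spoilage.
; TakePotion spawns a potion containing a proportional share of the mix.
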(event `self.ReceiveBeginPlay`
  (bind _aslabel_widget (cast `/Game/Blueprints/Environment/Labels/Widgets/LabelWidget` (`WidgetComponent.GetWidget` (`self.IngredientsWidget`))))
  (bind _output_get (set `self.IngredientsWidgetRef` _aslabel_widget))
  (set `/Game/Blueprints/Environment/Labels/Widgets/LabelWidget.Owner` self _output_get))

(event `self.ContentCollider.OnComponentBeginOverlap`
  (params (OverlappedComponent :type "PrimitiveComponent Object Reference") (OtherActor :type "Actor Object Reference") (OtherComp :type "PrimitiveComponent Object Reference") (OtherBodyIndex :type Integer) (bFromSweep :type Boolean) (SweepResult :type "HitResult Structure (by ref)"))
  (bind _asbp_world_ingredient_base (cast `/Game/Blueprints/Hero/WorldIngredients/BP_WorldIngredientBase` OtherActor)
    (:`then`
      (`self.AddIngredients` (`/Game/Blueprints/Hero/WorldIngredients/BP_WorldIngredientBase.Ingredients` _asbp_world_ingredient_base)
        (:`then_2`
          _)))
    (:`CastFailed`
      (bind _asbp_potion (cast `/Game/Blueprints/Hero/BP_Potion` OtherActor))
      (`self.AddIngredients` (`/Game/Blueprints/Hero/BP_Potion.Ingredients` _asbp_potion)
        (:`then_2`
          _))))
  (`self.K2_DestroyActor` OtherActor))

(event `self.ReceiveTick`
  (params (DeltaSeconds :type "Float (single-precision)"))
  (bind _ingredients (`self.Ingredients`))
  (bind _recipes (`self.Recipes`))
  (`|ExecutionSequence`
    (:`then_0`
      (`self.InterpolateVolume` DeltaSeconds))
    (:`then_1`
      (`self.InterpolateColor` DeltaSeconds))
    (:`then_2`
      (`self.InterpolateTemperature` DeltaSeconds))
    (:`then_3`
      (`self.InterpolateBubbles` DeltaSeconds))
    (:`then_4`
      (`self.SetUIParameters`))
    (:`then_5`
      (`self.SetTemperatureEffects`))
    (:`then_6`
      (if (> (`KismetArrayLibrary.Array_Length` _recipes) 0)
        (`self.CheckIngredients` (`KismetArrayLibrary.Array_Random` _recipes))))
    (:`then_7`
      (if (> (`KismetArrayLibrary.Array_Length` _ingredients) 0)
        (`self.CheckTemperature` (`KismetArrayLibrary.Array_Random` _ingredients))))))

(event `self.FireCollider.OnComponentBeginOverlap`
  (params (OverlappedComponent :type "PrimitiveComponent Object Reference") (OtherActor :type "Actor Object Reference") (OtherComp :type "PrimitiveComponent Object Reference") (OtherBodyIndex :type Integer) (bFromSweep :type Boolean) (SweepResult :type "HitResult Structure (by ref)"))
  (bind _asbp_fire_wood (cast `/Game/Blueprints/Hero/BP_FireWood` OtherActor)
    (:`then`
      (`self.AddFuel` (`/Game/Blueprints/Hero/BP_FireWood.HeatGain` _asbp_fire_wood)))
    (:`CastFailed`
      (cast `/Game/Blueprints/Hero/WorldIngredients/BP_Water` OtherActor)
      (`self.Extinguish`)))
  (`self.K2_DestroyActor` OtherActor))

(fn `AddIngredient`
  (params (Ingredient :type "/Game/Blueprints/Hero/Ingredients/IngredientPackage Structure"))
  (bind (_ingredient _volume) (break `/Game/Blueprints/Hero/Ingredients/IngredientPackage` Ingredient))
  (bind _ingredients (`self.Ingredients`))
  (for (_array_element _array_index) _ingredients
    (bind (_ingredient_2 _volume_2) (break `/Game/Blueprints/Hero/Ingredients/IngredientPackage` _array_element))
    (if (== _ingredient_2 _ingredient)
      (bind _structout (setmembers `/Game/Blueprints/Hero/Ingredients/IngredientPackage` :`StructRef` _array_element :`Volume` (+ _volume_2 _volume)))
      (`KismetArrayLibrary.Array_Set` (`self.Ingredients`) _array_index _structout)
      (return)))
  (`KismetArrayLibrary.Array_Add` _ingredients Ingredient))

(fn `BubbleBoost`
  (set `self.CurrentBubbleBoost` (`self.MaxBubbleBoost`)))

(fn `CheckIngredients`
  (params (Recipe :type "/Game/Blueprints/Hero/Recipes/BP_RecipeBase Class Reference"))
  (locals (HasAllIngredients :type Boolean :default true) (MinimumVolume :type "Float (double-precision)"))
  (bind (_ingredients _result _producetemperature) (defaults `Object` Recipe))
  (for _array_element _ingredients
    (bind _hasingredient (`self.HasIngredient` _array_element))
    (set `local.HasAllIngredients` (and (`local.HasAllIngredients`) _hasingredient)))
  (if (and (`local.HasAllIngredients`) (< _producetemperature (`self.Temperature`)))
    (`self.ProduceRecipe` Recipe)))

(fn `CheckTemperature`
  (params (Ingredient :type "/Game/Blueprints/Hero/Ingredients/IngredientPackage Structure (by ref)"))
  (bind _ingredient (break `/Game/Blueprints/Hero/Ingredients/IngredientPackage` Ingredient))
  (bind _temperature (`self.Temperature`))
  (bind (_color _ruintemperature _ruinresult) (defaults `Object` _ingredient))
  (bind _returnvalue (* (/ _temperature _ruintemperature) (`GameplayStatics.GetWorldDeltaSeconds`)))
  (if (`.ReturnValue` (`BlueprintMapLibrary.Map_Find` (`self.IngredientMap`) _ingredient))
    (if (> _temperature _ruintemperature)
      (`self.TakeIngredient` (make `/Game/Blueprints/Hero/Ingredients/IngredientPackage` _ingredient _returnvalue))
      (if (`KismetSystemLibrary.IsValidClass` _ruinresult)
        (`self.AddIngredient` (make `/Game/Blueprints/Hero/Ingredients/IngredientPackage` _ruinresult _returnvalue))
        (`self.ConsolidateContents`)))))

(fn `ClearCauldron`
  (`|ExecutionSequence`
    (:`then_0`
      (`KismetArrayLibrary.Array_Clear` (`self.Ingredients`)))
    (:`then_1`
      (`self.ConsolidateContents`))
    (:`then_2`
      (set `self.TargetColor` (struct :`R` 1.0 :`G` 1.0 :`B` 1.0 :`A` 1.0)))
    (:`then_3`
      (`FMODBlueprintStatics.PlayEventAttached` "/Game/FMOD/Events/SFX/Splash/Water_Splash_Random.Water_Splash_Random" (`self.Offset`) "None" (0.0 0.0 0.0) "KeepRelativeOffset"))))

(fn `ConsolidateContents`
  (`BlueprintMapLibrary.Map_Clear` (`self.IngredientMap`))
  (set `self.TargetVolume` 0.0)
  (for (_array_element _array_index) (`self.Ingredients`)
    (`self.RemoveIfEmpty` _array_element _array_index
      (:`NotRemoved`
        (`|ExecutionSequence`
          (:`then_0`
            (bind (_ingredient _volume) (break `/Game/Blueprints/Hero/Ingredients/IngredientPackage` _array_element))
            (`self.AddToIngredientMap` _ingredient _array_index))
          (:`then_1`
            (bind _output_get (set `self.TargetVolume` (+ _volume (`self.TargetVolume`))))
            (set `self.TargetColor` (`KismetMathLibrary.LinearColorLerp` (`self.TargetColor`) (defaults `Object` _ingredient) (/ _volume _output_get))))))
      (:`Removed`
        (`self.ConsolidateContents`))))
  (`/Game/Blueprints/Environment/Labels/Widgets/LabelWidget.UpdateList` (`self.IngredientsWidgetRef`) (`self.Ingredients`)))

(fn `HasIngredient`
  (params (Ingredient :type "/Game/Blueprints/Hero/Ingredients/IngredientPackage Structure"))
  (returns (HasIngredient :type Boolean) (Volume :type "Float (double-precision)"))
  (bind (_ingredient _volume) (break `/Game/Blueprints/Hero/Ingredients/IngredientPackage` Ingredient))
  (bind (_value _returnvalue) (`BlueprintMapLibrary.Map_Find` (`self.IngredientMap`) _ingredient))
  (bind (_ingredient_2 _volume_2) (break `/Game/Blueprints/Hero/Ingredients/IngredientPackage` (`|GetArrayItem` (`self.Ingredients`) _value)))
  (if _returnvalue
    (return (>= _volume_2 _volume) _volume_2)
    (else
      (return false 0.0))))

(fn `ProduceRecipe`
  (params (Recipe :type "/Game/Blueprints/Hero/Recipes/BP_RecipeBase Class Reference"))
  (bind (_ingredients _result) (defaults `Object` Recipe))
  (for _array_element _ingredients
    (`self.TakeIngredient` _array_element))
  (`self.AddIngredient` _result)
  (`self.ConsolidateContents`))

(fn `RemoveIngredient`
  (params (Ingredient :type "/Game/Blueprints/Hero/Ingredients/IngredientPackage Structure"))
  (bind (_value _returnvalue) (`BlueprintMapLibrary.Map_Find` (`self.IngredientMap`) (`.Ingredient_14_599B7E1D4295260D79700AAF58996B9A` (break `/Game/Blueprints/Hero/Ingredients/IngredientPackage` Ingredient))))
  (if _returnvalue
    (`KismetArrayLibrary.Array_Remove` (`self.Ingredients`) _value)
    (`self.ConsolidateContents`)
    (return)))

(fn `SetContentColor`
  (params (Color :type "LinearColor Structure"))
  (bind _returnvalue (`KismetMathLibrary.Conv_LinearColorToVector` Color))
  (`LightComponent.SetLightColor` (`self.PointLight`) Color true)
  (bind _asbp_cauldron_surface (cast `/Game/Blueprints/Hero/Cauldron/BP_CauldronSurface` (`ChildActorComponent.ChildActor` (`self.BP_CauldronSurface`))))
  (`MeshComponent.SetVectorParameterValueOnMaterials` (`/Game/FluidNinjaLive/NinjaLive.TraceMesh` _asbp_cauldron_surface) "FlowMapColor" _returnvalue)
  (`FXSystemComponent.SetVectorParameter` (`self.Bubbles`) "Color" _returnvalue))

(fn `SetContentScale`
  (params (Alpha :type "Float (double-precision)"))
  (`SceneComponent.SetWorldScale3D` (`self.Scaler`) (`KismetMathLibrary.MakeVector` 1.0 1.0 (`KismetMathLibrary.FClamp` Alpha 0.05))))

(fn `SetFireIntensity`
  (params (Alpha :type "Float (double-precision)"))
  (`LightComponent.SetIntensity` (`self.FireLight`) (* Alpha (`self.MaxFireLightIntensity`)))
  (`LightComponent.SetIntensity` (`self.FireLight3`) (* Alpha (`self.MaxFireLightIntensity`)))
  (`LightComponent.SetIntensity` (`self.FireLight2`) (* Alpha (`self.MaxFireLightIntensity`)))
  (`LightComponent.SetIntensity` (`self.FireLight1`) (* Alpha (`self.MaxFireLightIntensity`)))
  (`MaterialInstanceDynamic.SetScalarParameterValue` (`self.Flames`) "FlameIntensity" Alpha))

(fn `SetLightIntensity`
  (params (Alpha :type "Float (double-precision)"))
  (`LightComponent.SetIntensity` (`self.PointLight`) (* Alpha (`self.MaxLightIntensity`))))

(fn `SetVolume`
  (params (Liters :type "Float (double-precision)"))
  (bind _output_get (set `self.TargetVolume` Liters))
  (`self.SetContentScale` (/ _output_get (`self.MaxVolume`))))

(fn `TakeIngredient`
  (params (Ingredient :type "/Game/Blueprints/Hero/Ingredients/IngredientPackage Structure"))
  (bind _ingredient (break `/Game/Blueprints/Hero/Ingredients/IngredientPackage` Ingredient))
  (bind _ingredients (`self.Ingredients`))
  (bind (_value _returnvalue) (`BlueprintMapLibrary.Map_Find` (`self.IngredientMap`) _ingredient))
  (bind _output (`|GetArrayItem` _ingredients _value))
  (if _returnvalue
    (bind _structout (setmembers `/Game/Blueprints/Hero/Ingredients/IngredientPackage` :`StructRef` _output :`Volume` (- (`.Volume_17_17370D314A91F014C82054833DB75558` (break `/Game/Blueprints/Hero/Ingredients/IngredientPackage` _output)) (`.Volume_17_17370D314A91F014C82054833DB75558` (break `/Game/Blueprints/Hero/Ingredients/IngredientPackage` Ingredient)))))
    (`KismetArrayLibrary.Array_Set` _ingredients _value _structout)
    (`self.ConsolidateContents`)
    (else
      (`KismetSystemLibrary.PrintText` (`|FormatText` "CAULDRON ERROR: Tried to take non-cauldronized ingredient {Ingredient}!" (`KismetSystemLibrary.GetClassDisplayName` _ingredient))))))

(fn `TakePotion`
  (locals (PotionRatio :type "Float (double-precision)") (PotionIngredients :type "Array of /Game/Blueprints/Hero/Ingredients/IngredientPackage Structure"))
  (set `local.PotionRatio` (/ (`self.PotionSize`) (`self.TargetVolume`)))
  (for _array_element (`self.Ingredients`)
    (`|ExecutionSequence`
      (:`then_0`
        (bind (_ingredient _volume) (break `/Game/Blueprints/Hero/Ingredients/IngredientPackage` _array_element))
        (bind _ingredientpackage (make `/Game/Blueprints/Hero/Ingredients/IngredientPackage` _ingredient (* _volume (`local.PotionRatio`))))
        (`KismetArrayLibrary.Array_Add` (`local.PotionIngredients`) _ingredientpackage))
      (:`then_1`
        (`self.TakeIngredient` _ingredientpackage))))
  (`|ExecutionSequence`
    (:`then_0`
      (bind _returnvalue (`|SpawnActorFromClass` "/Game/Blueprints/Hero/BP_Potion.BP_Potion_C" (`KismetMathLibrary.ComposeTransforms` (`self.PotionSpawnLocation`) (`self.GetTransform`)) "Undefined" "OverrideRootScale" null (`local.PotionIngredients`) (`self.PotionSize`) null))
      (`FMODBlueprintStatics.PlayEventAttached` "/Game/FMOD/Events/SFX/Splash/Water_Splash_Random.Water_Splash_Random" (`Actor.RootComponent` _returnvalue) "None" (0.0 0.0 0.0) "KeepRelativeOffset"))
    (:`then_1`
      (`self.ConsolidateContents`))))

(fn `UserConstructionScript`
  (set `self.MaxLightIntensity` (`LightComponentBase.Intensity` (`self.PointLight`)))
  (bind _returnvalue (`PrimitiveComponent.CreateDynamicMaterialInstance` (`self.Cauldron`) 1 "/Game/Art/Hero/Kettle/M_Flames_Inst.M_Flames_Inst" "None"))
  (set `self.Flames` _returnvalue))