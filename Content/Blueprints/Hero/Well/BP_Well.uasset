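; BP_Well is an interactive well that lets the player sober up.
; Clicking it spawns an actor at the water spawn location, relative to the well, and plays a random splash sound attached to the SMHink component.
; Its consume event casts the player to BP_TomteCharacter, calls ConsumeEffect, resets drunkenness to zero and plays a 2D clunk sound.
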(event `self.OnClick`
  (`|SpawnActorFromClass` "/Game/Blueprints/Hero/WorldIngredients/BP_Water.BP_Water_C" (`KismetMathLibrary.ComposeTransforms` (`self.WaterSpawnLocation`) (`self.GetTransform`)) "Undefined" "OverrideRootScale" null null)
  (`FMODBlueprintStatics.PlayEventAttached` "/Game/FMOD/Events/SFX/Splash/Water_Splash_Random.Water_Splash_Random" (`self.SM_hink`) "None" (0.0 0.0 0.0) "KeepRelativeOffset"))

(event `/Game/Blueprints/Player/IConsumable.OnConsume`
  (bind _asbp_tomte_character (cast `/Game/Blueprints/Player/BP_TomteCharacter` (`GameplayStatics.GetPlayerCharacter` 0)))
  (`/Game/Blueprints/Player/BP_TomteCharacter.ConsumeEffect` _asbp_tomte_character 0)
  (`/Game/Blueprints/Player/BP_TomteCharacter.SetDrunkness` _asbp_tomte_character 0.0)
  (`FMODBlueprintStatics.PlayEvent2D` "/Game/FMOD/Events/Actors/Player/Player_Clunk.Player_Clunk"))

(fn `UserConstructionScript`)