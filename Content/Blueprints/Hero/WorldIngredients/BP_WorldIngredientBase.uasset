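; Base Blueprint for world ingredients that the player's Tomte character can consume, with an outline shown while hovered.
; On consume, it constructs an object from each entry's ingredient class and applies its effect to the character at full strength.
; It then plays a 2D burp sound event and destroys itself.
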(event `/Game/Blueprints/Player/IConsumable.OnConsume`
  (for _array_element (`self.Ingredients`)
    (bind _returnvalue (`|GenericCreateObject` self (`.Ingredient_14_599B7E1D4295260D79700AAF58996B9A` (break `/Game/Blueprints/Hero/Ingredients/IngredientPackage` _array_element))))
    (bind _asbp_tomte_character (cast `/Game/Blueprints/Player/BP_TomteCharacter` (`GameplayStatics.GetPlayerCharacter` 0)))
    (`/Game/Blueprints/Hero/Ingredients/BP_IngredientBase.Consume` _returnvalue _asbp_tomte_character 1.0))
  (`FMODBlueprintStatics.PlayEvent2D` "/Game/FMOD/Events/Actors/Player/Player_Burp.Player_Burp")
  (`self.K2_DestroyActor`))

(event `/Game/Blueprints/Player/IInteractible.OnHoverBegin`
  (`/Game/Blueprints/Libraries/BPL_InteractionFunctions.SetOutline` self true (`self.OutlineColor`)))

(event `/Game/Blueprints/Player/IInteractible.OnHoverEnd`
  (`/Game/Blueprints/Libraries/BPL_InteractionFunctions.SetOutline` self false (`self.OutlineColor`)))

(fn `UserConstructionScript`)