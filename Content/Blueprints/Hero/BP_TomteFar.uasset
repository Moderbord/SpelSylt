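; BP_TomteFar is a rocking tomte grandfather NPC who requests potions and judges those brought to him.
; A recipe widget shows his current desire from an ordered list, which advances on success and stops at the last.
; A potion entering GiftCollider passes if the desired ingredient's volume share exceeds DesiredPotency, then is destroyed either way.
; Success or failure plays a voice event and flashes the point light in a matching color, alongside a burp.
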(event `self.ReceiveBeginPlay`
  (bind _defaultsceneroot (`self.DefaultSceneRoot`))
  (`|ExecutionSequence`
    (:`then_0`
      (`LightComponent.SetIntensity` (`self.PointLight`) 0.0))
    (:`then_1`
      (bind _asrecipe_widget (cast `/Game/Blueprints/UI/RecipeWidget` (`WidgetComponent.GetWidget` (`self.RecipeWidget`))))
      (`/Game/Blueprints/UI/RecipeWidget.Set Child Variables` _asrecipe_widget self (`self.FadeDistance`)))
    (:`then_2`
      (`self.AdvanceDesire`))
    (:`then_3`
      (`FMODBlueprintStatics.PlayEventAttached` "/Game/FMOD/Events/Actors/Farfar/Farfar_Mumel.Farfar_Mumel" _defaultsceneroot "None" (0.0 0.0 0.0) "KeepRelativeOffset")
      (`FMODBlueprintStatics.PlayEventAttached` "/Game/FMOD/Events/SFX/Farfar_Chair.Farfar_Chair" _defaultsceneroot "None" (0.0 0.0 0.0) "KeepRelativeOffset"))))

(event `self.ReceiveTick`
  (params (DeltaSeconds :type "Float (single-precision)"))
  (`SceneComponent.K2_SetRelativeRotation` (`self.TomteOffset`) (`KismetMathLibrary.MakeRotator` (* (`KismetMathLibrary.Sin` (* (`KismetSystemLibrary.GetGameTimeInSeconds`) (`self.GungSpeed`))) (`self.GungRotation`))) false false))

(event `self.GiftCollider.OnComponentBeginOverlap`
  (params (OverlappedComponent :type "PrimitiveComponent Object Reference") (OtherActor :type "Actor Object Reference") (OtherComp :type "PrimitiveComponent Object Reference") (OtherBodyIndex :type Integer) (bFromSweep :type Boolean) (SweepResult :type "HitResult Structure (by ref)"))
  (bind _asbp_potion (cast `/Game/Blueprints/Hero/BP_Potion` OtherActor))
  (`|ExecutionSequence`
    (:`then_0`
      (bind _success (`self.CheckIngredients` _asbp_potion))
      (if _success
        (`self.Succeed`)
        (else
          (`self.Fail`))))
    (:`then_1`
      (`FMODBlueprintStatics.PlayEventAttached` "/Game/FMOD/Events/Actors/Player/Burp/Burp.Burp" (`self.MouthLocation`) "None" (0.0 0.0 0.0) "KeepRelativeOffset"))
    (:`then_2`
      (`self.K2_DestroyActor` _asbp_potion))))

(fn `CheckIngredients`
  (params (Potion :type "/Game/Blueprints/Hero/BP_Potion Object Reference"))
  (returns (Success :type Boolean))
  (locals (TempSuccess :type Boolean))
  (for _array_element (`/Game/Blueprints/Hero/BP_Potion.Ingredients` Potion)
    (bind (_ingredient _volume) (break `/Game/Blueprints/Hero/Ingredients/IngredientPackage` _array_element))
    (if (and (== (`self.GetCurrentDesire`) _ingredient) (> (/ _volume (`/Game/Blueprints/Hero/BP_Potion.Volume` Potion)) (`self.DesiredPotency`)))
      (set `local.TempSuccess` true)))
  (return (`local.TempSuccess`)))

(fn `GetCurrentDesire`
  (returns (Output :type "/Game/Blueprints/Hero/Ingredients/BP_IngredientBase Class Reference"))
  (bind _output_get (set `self.DesireIndex` (`self.DesireIndex`)))
  (return (`.Ingredient_14_599B7E1D4295260D79700AAF58996B9A` (break `/Game/Blueprints/Hero/Ingredients/IngredientPackage` (`.Result` (defaults `Object` (`|GetArrayItem` (`self.Desires`) _output_get)))))))

(fn `UserConstructionScript`
  (set `self.LightIntensity` (`LightComponentBase.Intensity` (`self.PointLight`))))