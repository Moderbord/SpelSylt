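; BP_Loader is a test actor for custom compute shader nodes.
; Every Tick it runs a base material compute shader with its Material and actor location.
; Unconnected chains hold further tests: a render-target material shader, a result print, and nested async base and Pi-estimation shaders.
; The construction script stores a hard-coded triangle with its calculated normals and tangents, but builds no mesh from them.
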(event `self.ReceiveTick`
  (params (DeltaSeconds :type "Float (single-precision)"))
  (bind _value (`SimpleMaterialTestLibrary_AsyncExecution.ExecuteBaseMaterialComputeShader` self (`self.Material`) (`self.K2_GetActorLocation`))))

(fn `UserConstructionScript`
  (bind _output_get (set `self.Vertices` (`|MakeArray` (0.0 0.0 0.0) (0.0 0.0 200.0) (200.0 0.0 0.0) :!type "Vector Structure")))
  (bind _output_get_2 (set `self.Triangles` (`|MakeArray` 2 1 0)))
  (bind (_normals _tangents) (`KismetProceduralMeshLibrary.CalculateTangentsForMesh` _output_get _output_get_2))
  (set `self.Tangents` _tangents)
  (set `self.Normals` _normals))