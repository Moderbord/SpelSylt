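; First-person Tomte player character with movement, mouse look and physics object grabbing.
; Tick line-traces from the camera for physics bodies, caching the hit and sending hover or trace-end messages to I_Grabbable actors.
; Fire holds simulating components via a physics constraint to a slot, optionally eased to its default position and shifted by mouse wheel.
; Poke releases the held object and applies a camera-forward impulse to the traced hit.
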(event `self.ReceiveTick`
  (params (DeltaSeconds :type "Float (single-precision)"))
  (bind _hit (`self.Trace`)
    (:`_`
      (if _hit
        (`self.HandleInterfaces`)
        (else
          (`self.HandleEnds`))))))

(event `self.ReceiveBeginPlay`
  (bind _returnvalue (`GameplayStatics.GetPlayerController` 0))
  (bind _sensitivity (`self.Sensitivity`))
  (set `PlayerController.InputPitchScale` _sensitivity _returnvalue)
  (bind _result (`/Engine/EditorBlueprintResources/StandardMacros.NegateFloat` _sensitivity)
    (:`  `
      (set `PlayerController.InputYawScale` _result _returnvalue))))

(event `InputAction|Fire`
  (params (Key :type "Key Structure"))
  (bind _heldobjectslot (`self.HeldObjectSlot`))
  (:`Pressed`
    (`/Engine/EditorBlueprintResources/StandardMacros.IsValid` (`self.HeldObject`)
      (:`Is Not Valid`
        (if (`self.Hit`)
          (`self.Grab` (`self.LastTraceHit`)
            (:`_`
              (if (not (`self.GrabInPlace`))
                (`KismetSystemLibrary.MoveComponentTo` _heldobjectslot (`SceneComponent.RelativeLocation` (`self.HeldObjectDefaultLocation`)) (`SceneComponent.RelativeRotation` _heldobjectslot) true true 0.3))))))))
  (:`Released`
    (`/Engine/EditorBlueprintResources/StandardMacros.IsValid` (`self.HeldObject`)
      (:`Is Valid`
        (`self.Drop`
          (:`_`
            (set `self.HeldObject` null)))))))

(event `InputAction|Poke`
  (params (Key :type "Key Structure"))
  (:`Pressed`
    (`/Engine/EditorBlueprintResources/StandardMacros.IsValid` (`self.HeldObject`)
      (:`Is Valid`
        (if (`self.Hit`)
          (`self.Drop`
            (:`_`
              (`self.Poke` (`self.LastTraceHit`)
                (:`_`
                  (set `self.HeldObject` null))))))))))

(event `InputAxis|Forward`
  (params (AxisValue :type "Float (single-precision)"))
  ;[1 1 1] MOVEMENT
  (`self.AddMovementInput` (`SceneComponent.GetForwardVector` (`self.CapsuleComponent`)) AxisValue))

(event `InputAxis|Right`
  (params (AxisValue :type "Float (single-precision)"))
  ;[1 1 1] MOVEMENT
  (`self.AddMovementInput` (`SceneComponent.GetRightVector` (`self.CapsuleComponent`)) AxisValue))

(event `InputAxis|Turn`
  (params (AxisValue :type "Float (single-precision)"))
  ;[1 1 1] MOVEMENT
  (`self.AddControllerYawInput` (* AxisValue (`self.Sensitivity`))))

(event `InputAxis|LookUp`
  (params (AxisValue :type "Float (single-precision)"))
  ;[1 1 1] MOVEMENT
  (`self.AddControllerPitchInput` (* AxisValue (`self.Sensitivity`))))

(event `InputAction|Jump`
  (params (Key :type "Key Structure"))
  ;[1 1 1] MOVEMENT
  (:`Pressed`
    (`self.Jump`))
  (:`Released`
    (`self.StopJumping`)))

(event `Key|MouseScrollUp`
  (params (Key :type "Key Structure"))
  (bind _heldobjectslot (`self.HeldObjectSlot`))
  (:`Pressed`
    (`SceneComponent.K2_SetRelativeLocation` _heldobjectslot (+ (`SceneComponent.RelativeLocation` _heldobjectslot) (25.0 0.0 0.0)) false false)))

(event `Key|MouseScrollDown`
  (params (Key :type "Key Structure"))
  (bind _heldobjectslot (`self.HeldObjectSlot`))
  (:`Pressed`
    (`SceneComponent.K2_SetRelativeLocation` _heldobjectslot (+ (`SceneComponent.RelativeLocation` _heldobjectslot) (-25.0 0.0 0.0)) false false)))

(fn `UserConstructionScript`)