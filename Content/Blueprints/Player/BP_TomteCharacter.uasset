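; First-person player character for a Tomte, with movement, physics grabbing and poking, a backpack, a carried lantern and consumable effects.
; Each tick a camera line trace finds physics objects, driving interface hover messages and feeding the grab, poke, pick-up and consume inputs.
; Held objects hang on a physics constraint, while backpack items are hidden until dropped together.
; Tick also applies drunkenness camera shake, lantern following and distance-based surface footsteps.
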(event `InputAction|ToggleLantern`
  (params (Key :type "Key Structure"))
  (:`Pressed`
    (if (`self.HasLantern`)
      (bind _isa (`/Engine/EditorBlueprintResources/StandardMacros.FlipFlop`)
        (:`A`
          _)
        (:`B`
          _))
      (`SceneComponent.SetVisibility` (`/Game/Art/Hero/Lantern/BP_Lantern.DefaultSceneRoot` (`self.Lantern`)) (not _isa) true))))

(event `InputAction|PlaceLantern`
  (params (Key :type "Key Structure")))

(event `SetDrunkness`
  (params (Drunkness :type "Float (double-precision)"))
  (set `self.Drunkness` Drunkness))

(event `self.ReceiveTick`
  (params (DeltaSeconds :type "Float (single-precision)"))
  (`PlayerController.ClientStartCameraShake` :`self` (`GameplayStatics.GetPlayerController` 0) :`Shake` "/Game/Blueprints/Player/DrunkShake.DrunkShake_C" :`Scale` (`self.Drunkness`))
  (`self.MoveSound`)
  (if (`self.HasLantern`)
    (`SceneComponent.K2_SetWorldLocationAndRotation` (`/Game/Art/Hero/Lantern/BP_Lantern.DefaultSceneRoot` (`self.Lantern`)) (`SceneComponent.K2_GetComponentLocation` (`self.LanternLocation`)) (`SceneComponent.K2_GetComponentRotation` (`self.CapsuleComponent`)) false false))
  (bind _hit (`self.Trace`)
    (:`_`
      (if _hit
        (`self.HandleInterfaces`)
        (else
          (`self.HandleEnds`))))))

(event `self.ReceiveBeginPlay`
  (bind _returnvalue (`GameplayStatics.GetPlayerController` 0))
  (bind _sensitivity (`self.Sensitivity`))
  (set `PlayerController.InputPitchScale` _sensitivity _returnvalue)
  (bind _result (`/Engine/EditorBlueprintResources/StandardMacros.NegateFloat` _sensitivity)
    (:`  `
      (set `PlayerController.InputYawScale` _result _returnvalue)
      (`PrimitiveComponent.SetCollisionResponseToChannel` (`self.CapsuleComponent`) "ECC_PhysicsBody" "ECR_Ignore")
      (set `self.LastSoundPos` (`SceneComponent.K2_GetComponentLocation` (`self.CapsuleComponent`)))
      (if (`self.EnableCrosshair`)
        (bind _returnvalue_2 (`|CreateWidget` "/Game/Blueprints/Player/Crosshair/CrosshairWidget.CrosshairWidget_C"))
        (bind _output_get (set `self.Crosshair` _returnvalue_2))
        (`UserWidget.AddToViewport` _output_get 0)))))

(event `InputAction|Fire`
  (params (Key :type "Key Structure"))
  (bind _heldobjectslot (`self.HeldObjectSlot`))
  (:`Pressed`
    (`/Engine/EditorBlueprintResources/StandardMacros.IsValid` (`self.HeldObject`)
      (:`Is Not Valid`
        (if (`self.Hit`)
          (`self.Grab` (`self.LastTraceHit`)
            (:`_`
              (if (not (`self.GrabInPlace`))
                (`KismetSystemLibrary.MoveComponentTo` _heldobjectslot (`SceneComponent.RelativeLocation` (`self.BackpackSpawnpoint`)) (`SceneComponent.RelativeRotation` _heldobjectslot) true true 0.3))))))))
  (:`Released`
    (`/Engine/EditorBlueprintResources/StandardMacros.IsValid` (`self.HeldObject`)
      (:`Is Valid`
        (`self.Drop`
          (:`_`
            (set `self.HeldObject` null)))))))

(event `InputAction|Poke`
  (params (Key :type "Key Structure"))
  (:`Pressed`
    (`/Engine/EditorBlueprintResources/StandardMacros.IsValid` (`self.HeldObject`)
      (:`Is Valid`
        (if (`self.Hit`)
          (`self.Drop`
            (:`_`
              (`self.Poke` (`self.LastTraceHit`)
                (:`_`
                  (set `self.HeldObject` null))))))))))

(event `InputAxis|Forward`
  (params (AxisValue :type "Float (single-precision)"))
  ;[1 1 1] MOVEMENT
  (`self.AddMovementInput` (`SceneComponent.GetForwardVector` (`self.CapsuleComponent`)) AxisValue))

(event `InputAxis|Right`
  (params (AxisValue :type "Float (single-precision)"))
  ;[1 1 1] MOVEMENT
  (`self.AddMovementInput` (`SceneComponent.GetRightVector` (`self.CapsuleComponent`)) AxisValue))

(event `InputAxis|Turn`
  (params (AxisValue :type "Float (single-precision)"))
  ;[1 1 1] MOVEMENT
  (`self.AddControllerYawInput` (* AxisValue (`self.Sensitivity`))))

(event `InputAxis|LookUp`
  (params (AxisValue :type "Float (single-precision)"))
  ;[1 1 1] MOVEMENT
  (`self.AddControllerPitchInput` (* AxisValue (`self.Sensitivity`))))

(event `InputAction|Consume`
  (params (Key :type "Key Structure"))
  (:`Pressed`
    (if (`self.Hit`)
      (message `/Game/Blueprints/Player/IConsumable.OnConsume` (`.HitActor` (`GameplayStatics.BreakHitResult` (`self.LastTraceHit`)))))))

(event `InputAction|Jump`
  (params (Key :type "Key Structure"))
  ;[1 1 1] MOVEMENT
  (:`Pressed`
    (`self.Jump`))
  (:`Released`
    (`self.StopJumping`)))

(event `Key|MouseScrollUp`
  (params (Key :type "Key Structure"))
  (bind _heldobjectslot (`self.HeldObjectSlot`))
  (:`Pressed`
    (`SceneComponent.K2_SetRelativeLocation` _heldobjectslot (+ (`SceneComponent.RelativeLocation` _heldobjectslot) (25.0 0.0 0.0)) false false)))

(event `InputAction|PickUp`
  (params (Key :type "Key Structure"))
  (bind (_bblockinghit _binitialoverlap _time _distance _location _impactpoint _normal _impactnormal _physmat _hitactor _hitcomponent) (`GameplayStatics.BreakHitResult` (`self.LastTraceHit`)))
  (:`Pressed`
    (if (`self.Hit`)
      (if (`KismetSystemLibrary.DoesImplementInterface` _hitactor "/Game/Blueprints/Player/IGrabbable.IGrabbable_C")
        (`|ExecutionSequence`
          (:`then_0`
            (message `/Game/Blueprints/Player/IGrabbable.OnTake` _hitactor))
          (:`then_1`
            (`self.AddToBackpack` _hitcomponent))
          (:`then_2`
            (`FMODBlueprintStatics.PlayEventAttached` "/Game/FMOD/Events/SFX/Bag/Bag_Handling.Bag_Handling" (`self.CapsuleComponent`) "None" (0.0 0.0 0.0) "KeepRelativeOffset")))))))

(event `Key|MouseScrollDown`
  (params (Key :type "Key Structure"))
  (bind _heldobjectslot (`self.HeldObjectSlot`))
  (:`Pressed`
    (`SceneComponent.K2_SetRelativeLocation` _heldobjectslot (+ (`SceneComponent.RelativeLocation` _heldobjectslot) (-25.0 0.0 0.0)) false false)))

(event `InputAction|DropAll`
  (params (Key :type "Key Structure"))
  (:`Pressed`
    (for _array_element (`self.BackpackComponents`)
      (`SceneComponent.K2_SetWorldLocation` _array_element (`self.RandomAreaVector` (`SceneComponent.K2_GetComponentLocation` (`self.BackpackSpawnpoint`))) false false)
      (`SceneComponent.SetVisibility` _array_element true true)
      (message `/Game/Blueprints/Player/IGrabbable.OnRelease` _array_element))
    (`|ExecutionSequence`
      (:`then_0`
        (`KismetArrayLibrary.Array_Clear` (`self.BackpackComponents`)))
      (:`then_1`
        (`FMODBlueprintStatics.PlayEventAttached` "/Game/FMOD/Events/SFX/Bag/Bag_Drop.Bag_Drop" (`self.CapsuleComponent`) "None" (0.0 0.0 0.0) "KeepRelativeOffset")))))

(event `Key|Escape`
  (params (Key :type "Key Structure"))
  (:`Pressed`
    (`KismetSystemLibrary.QuitGame` null "Quit")))

(event `ConsumeEffect`
  (params (PostEffect :type Integer))
  (set `PostProcessComponent.Settings` (select `int` PostEffect :`0` (`self.Defaul`) :`1` (`self.Flug`) :`2` (`self.Knark`) :`3` (`self.Magic`)) (`self.PostProcess`)))

(fn `MoveSound`
  (locals (NewLocalVar_0 :type "FindFloorResult Structure"))
  (bind _returnvalue (`SceneComponent.K2_GetComponentLocation` (`self.CapsuleComponent`)))
  (bind _currentfloor (`CharacterMovementComponent.CurrentFloor` (`self.CharacterMovement`)))
  (if (> (`KismetMathLibrary.VSize` (- _returnvalue (`self.LastSoundPos`))) (`self.MinDistanceSound`))
    (set `self.LastSoundPos` _returnvalue)
    (if (break `FindFloorResult` _currentfloor)
      (switch `EPhysicalSurface` (`PhysicalMaterial.SurfaceType` (`.PhysMat` (`GameplayStatics.BreakHitResult` (`.HitResult` (break `FindFloorResult` _currentfloor)))))
        (:`SurfaceType1`
          (`FMODBlueprintStatics.PlayEvent2D` "/Game/FMOD/Events/Actors/Player/Footsteps/Footsteps_Wood.Footsteps_Wood"))
        (:`SurfaceType4`
          (`FMODBlueprintStatics.PlayEvent2D` "/Game/FMOD/Events/Actors/Player/Footsteps/Footsteps_Grass.Footsteps_Grass"))
        (:`SurfaceType5`
          (`FMODBlueprintStatics.PlayEvent2D` "/Game/FMOD/Events/Actors/Player/Footsteps/Footsteps_Gravel.Footsteps_Gravel"))))))

(fn `UserConstructionScript`)